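; BP_InputReceiver listens for a player's start input and asks the game mode to spawn that player.
; After a one-second delay on BeginPlay, it adds the default Enhanced Input mapping context to the controller at its PlayerIndex.
; IA_Start sends SpawnPlayerMessage with the index and itself, guarded to fire once.
; IA_Start_2 shares that path only for player index 1, otherwise printing controller and index debug info.
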(event `self.ReceiveBeginPlay`
  ;[1 1 1] Input Mapping
  (`KismetSystemLibrary.Delay` 1.0)
  (bind _asmy_player_controller (cast `/Game/Core/Characters/Player/MyPlayerController` (`GameplayStatics.GetPlayerController` (`self.PlayerIndex`))))
  (bind _returnvalue (pcsubsystem `EnhancedInputLocalPlayerSubsystem` _asmy_player_controller))
  (`/Engine/EditorBlueprintResources/StandardMacros.IsValid` _returnvalue
    (:`Is Valid`
      (`EnhancedInputSubsystemInterface.AddMappingContext` _returnvalue "/Game/Core/Characters/Player/Input/IMC_Default.IMC_Default" 0 (struct)))))

(event `EnhancedInput|/Game/Core/Characters/Player/Input/Actions/IA_Start`
  (params (ActionValue :type Boolean) (ElapsedSeconds :type "Float (double-precision)") (TriggeredSeconds :type "Float (double-precision)") (InputAction :type "InputAction Object Reference" :default "/Game/Core/Characters/Player/Input/Actions/IA_Start.IA_Start"))
  (:`Started`
    (if (not (`self.doOnce`)) :!label _label
      (message `/Game/Core/GameFeatures/BPI_GameMode.SpawnPlayer` (`GameplayStatics.GetGameMode`) (`self.PlayerIndex`) self)
      (`KismetSystemLibrary.PrintString` "Hello")
      (set `self.doOnce` true))))

(event `EnhancedInput|/Game/Core/Characters/Player/Input/Actions/IA_Start_2`
  (params (ActionValue :type Boolean) (ElapsedSeconds :type "Float (double-precision)") (TriggeredSeconds :type "Float (double-precision)") (InputAction :type "InputAction Object Reference" :default "/Game/Core/Characters/Player/Input/Actions/IA_Start_2.IA_Start_2"))
  (bind _returnvalue (`GameplayStatics.GetPlayerController` (`self.PlayerIndex`)))
  (:`Started`
    (if (== (`self.PlayerIndex`) 1)
      (`KismetSystemLibrary.PrintString` (`KismetStringLibrary.Concat_StrStr` "" "PlayerIndex = " (`KismetStringLibrary.Conv_IntToString` (`self.PlayerIndex`)) " : Output by : " (`KismetSystemLibrary.GetDisplayName` self)) false)
      (goto _label)
      (else
        (bind _playerindex (`TurnBasedBlueprintLibrary.GetMyPlayerIndex` _returnvalue))
        (`KismetSystemLibrary.PrintString` (`KismetStringLibrary.Concat_StrStr` " : Output by : " (`KismetSystemLibrary.GetDisplayName` self) " : PlayerIndex = " (`KismetStringLibrary.Conv_IntToString` (`self.PlayerIndex`)) " : PlayerController = " (`KismetSystemLibrary.GetDisplayName` _returnvalue) ".GetMyPlayerIndex = " (`KismetStringLibrary.Conv_IntToString` _playerindex)) false)))))

(fn `UserConstructionScript`)