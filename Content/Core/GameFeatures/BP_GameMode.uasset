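; Game mode that sets up local multiplayer by creating a player and input receiver for each index-tagged PlayerStart.
; On BeginPlay it gathers PlayerStarts and matches their integer tags to array indices.
; Each match spawns a possessed BP_InputReceiver at the start in that array slot, not necessarily the tagged one, and records it with its controller.
; SpawnPlayer later swaps possession to a BP_PlayerCharacter spawned at the receiver's transform.
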(event `self.ReceiveBeginPlay`
  (`self.GetPlayerStartPoints`)
  (`self.SpawnInputReceivers`))

(fn `GetPlayerStartPoints`
  (bind _outactors (`GameplayStatics.GetAllActorsOfClass` "/Script/Engine.PlayerStart"))
  (set `self.PlayerStartArray` _outactors))

(fn `Pure_NameToInt`
  (params (PlayerStart :type "PlayerStart Object Reference"))
  (returns (ReturnValue :type Integer))
  (return (`KismetStringLibrary.Conv_StringToInt` (`KismetStringLibrary.Conv_NameToString` (`PlayerStart.PlayerStartTag` PlayerStart)))))

(fn `SpawnInputReceivers`
  (bind _returnvalue (`GameplayStatics.GetPlayerController` (`self.Array Index`)))
  (for (_ _array_index) (`self.PlayerStartArray`)
    (set `self.Array Index` _array_index)
    (for _array_element (`self.PlayerStartArray`)
      (if (== (`self.Pure_NameToInt` _array_element) (`self.Array Index`))
        (`GameplayStatics.CreatePlayer` (`self.Array Index`))
        (bind _returnvalue_2 (`|SpawnActorFromClass` "/Game/Core/GameFeatures/BP_InputReceiver.BP_InputReceiver_C" (`self.GetTransform` (`|GetArrayItem` (`self.PlayerStartArray`) (`self.Array Index`))) "Undefined" "OverrideRootScale" null (`self.Array Index`) null))
        (`KismetArrayLibrary.Array_AddUnique` (`self.InputReceiverArray`) _returnvalue_2)
        (`Controller.Possess` _returnvalue _returnvalue_2)
        (`KismetArrayLibrary.Array_AddUnique` (`self.ControllerArray`) _returnvalue)))))

(fn `SpawnPlayer`
  (params (CurrentPlayerIndex :type Integer) (InputReceiver :type "/Game/Core/GameFeatures/BP_InputReceiver Object Reference"))
  (returns (Return :type Boolean))
  (bind _returnvalue (`|SpawnActorFromClass` "/Game/Core/Characters/Player/BP_PlayerCharacter.BP_PlayerCharacter_C" (`self.GetTransform` InputReceiver) "Undefined" "OverrideRootScale" null CurrentPlayerIndex null))
  (`Controller.Possess` (`GameplayStatics.GetPlayerController` CurrentPlayerIndex) _returnvalue)
  (return false))

(fn `UserConstructionScript`)