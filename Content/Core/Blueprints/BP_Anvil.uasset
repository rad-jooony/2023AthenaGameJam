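; Anvil crafting station that turns molten iron and wood sticks into a great sword, sword or spear.
; Each tick it updates its widget, calls a start-of-tick routine and runs Crafting if ingredients are present.
; Crafting tallies ingredients by class-name string, picks the first matching recipe in that priority order and queues the weapon name in Processed.
; DeleteIngredients then removes the used entries from the Ingredients array.
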(event `self.ReceiveTick`
  (params (DeltaSeconds :type "Float (single-precision)"))
  (`self.UpdateWidget`)
  (`self.CALL_AT_START_OF_TICK`)
  (bind _out (`self.IsIngredientsEmpty`))
  (if (not _out)
    (`self.Crafting`)))

(fn `Crafting`
  (locals (iron :type Integer) (sticks :type Integer))
  (for _array_element (`self.Ingredients`)
    (if (`KismetStringLibrary.EqualEqual_StrStr` _array_element "BP_MoltenIron_C")
      (set `local.iron` (+ (`local.iron`) 1))
      (elif (`KismetStringLibrary.EqualEqual_StrStr` _array_element "BP_WoodStick_C")
        (set `local.sticks` (+ (`local.sticks`) 1)))))
  (if (and (>= (`local.iron`) 3) (>= (`local.sticks`) 1))
    (bind _output_get (set `self.NameOfProcessedMaterialToOutput` "BP_GreatSword_C"))
    (`KismetArrayLibrary.Array_Add` (`self.Processed`) _output_get)
    (`self.DeleteIngredients` 3 "BP_MoltenIron_C")
    (set `local.iron` (- (`local.iron`) 3))
    (`self.DeleteIngredients` 1 "BP_WoodStick_C")
    (set `local.sticks` (- (`local.sticks`) 1))
    (elif (and (>= (`local.iron`) 2) (>= (`local.sticks`) 1))
      (bind _output_get_2 (set `self.NameOfProcessedMaterialToOutput` "BP_Sword_C"))
      (`KismetArrayLibrary.Array_Add` (`self.Processed`) _output_get_2)
      (`self.DeleteIngredients` 2 "BP_MoltenIron_C")
      (set `local.iron` (- (`local.iron`) 2))
      (`self.DeleteIngredients` 1 "BP_WoodStick_C")
      (set `local.sticks` (- (`local.sticks`) 1))
      (elif (and (>= (`local.iron`) 1) (>= (`local.sticks`) 2))
        (bind _output_get_3 (set `self.NameOfProcessedMaterialToOutput` "BP_Spear_C"))
        (`KismetArrayLibrary.Array_Add` (`self.Processed`) _output_get_3)
        (`self.DeleteIngredients` 1 "BP_MoltenIron_C")
        (set `local.iron` (- (`local.iron`) 1))
        (`self.DeleteIngredients` 2 "BP_WoodStick_C")
        (set `local.sticks` (- (`local.sticks`) 2))))))

(fn `DeleteIngredients`
  (params (AmountToDelete :type Integer) (IngredientToDelete :type String))
  (locals (i :type Integer))
  (for (_array_element _array_index) (`self.Ingredients`)
    (if (`KismetStringLibrary.EqualEqual_StrStr` _array_element IngredientToDelete)
      (`KismetArrayLibrary.Array_Remove` (`self.Ingredients`) _array_index)
      (bind _output_get (set `local.i` (+ (`local.i`) 1)))
      (if (== _output_get AmountToDelete)
        (break)))))

(fn `UserConstructionScript`)