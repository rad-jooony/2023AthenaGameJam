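; BP_ItemHolder is a holder actor that stores one item class and displays it as a spawned actor.
; Its collider sets IsOverlapping while a BP_PlayerCharacter is inside.
; AddItemToStoredItem, only when empty, stores the class, spawns it at the ItemOnTable location, keeps the reference and prints a debug string.
; RemoveFromStoredItem clears the stored class and destroys the spawned actor.
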(event `self.Collider.OnComponentBeginOverlap`
  (params (OverlappedComponent :type "PrimitiveComponent Object Reference") (OtherActor :type "Actor Object Reference") (OtherComp :type "PrimitiveComponent Object Reference") (OtherBodyIndex :type Integer) (bFromSweep :type Boolean) (SweepResult :type "HitResult Structure (by ref)"))
  (cast `/Game/Core/Characters/Player/BP_PlayerCharacter` OtherActor)
  (set `self.IsOverlapping` true))

(event `self.Collider.OnComponentEndOverlap`
  (params (OverlappedComponent :type "PrimitiveComponent Object Reference") (OtherActor :type "Actor Object Reference") (OtherComp :type "PrimitiveComponent Object Reference") (OtherBodyIndex :type Integer))
  (cast `/Game/Core/Characters/Player/BP_PlayerCharacter` OtherActor)
  (set `self.IsOverlapping` false))

(fn `AddItemToStoredItem`
  (params (ItemToAdd :type "/Game/Core/Blueprints/BP_PickupItem Class Reference"))
  (`self.IsStoredItemEmpty`
    (:`true`
      (bind _output_get (set `self.StoredItem` ItemToAdd))
      (bind _returnvalue (`|SpawnActorFromClass` _output_get (`KismetMathLibrary.MakeTransform` (`SceneComponent.K2_GetComponentLocation` (`self.ItemOnTable`))) "Undefined" "OverrideRootScale" null null))
      (set `self.ItemOnTableVar` _returnvalue)
      (`KismetSystemLibrary.PrintString` "Hello"))))

(fn `RemoveFromStoredItem`
  (set `self.StoredItem` null)
  (`self.K2_DestroyActor` (`self.ItemOnTableVar`))
  (set `self.ItemOnTableVar` null))

(fn `UserConstructionScript`)