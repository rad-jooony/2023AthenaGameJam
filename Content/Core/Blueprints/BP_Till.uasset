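; BP_Till is the till that takes customer orders.
; When a BP_Customer begins overlapping its Collider, it appends that customer's MyOrder to its OrderList.
; A separate ADD_TEST_ORDER debug function appends a test order, then prints the class display name of every entry in the list.
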(event `self.Collider.OnComponentBeginOverlap`
  (params (OverlappedComponent :type "PrimitiveComponent Object Reference") (OtherActor :type "Actor Object Reference") (OtherComp :type "PrimitiveComponent Object Reference") (OtherBodyIndex :type Integer) (bFromSweep :type Boolean) (SweepResult :type "HitResult Structure (by ref)"))
  (bind _asbp_customer (cast `/Game/Core/Blueprints/BP_Customer` OtherActor))
  (`KismetArrayLibrary.Array_Append` (`self.OrderList`) (`/Game/Core/Blueprints/BP_Customer.MyOrder` _asbp_customer)))

(fn `ADD_TEST_ORDER`
  (bind _orderlist (`self.OrderList`))
  (`KismetArrayLibrary.Array_Append` _orderlist (`self.TEST_ORDER`))
  (for _array_element _orderlist
    (`KismetSystemLibrary.PrintString` (`KismetSystemLibrary.GetClassDisplayName` _array_element))))

(fn `UserConstructionScript`)