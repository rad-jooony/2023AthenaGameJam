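; BP_Caster is a converter actor that displays the mould currently selected for casting as a spawned actor.
; Each Tick updates the widget, runs a start-of-tick hook, then looks up CurrentMould in FancyMap for the class to spawn.
; For spear head, blade or big blade moulds, it destroys the previous MouldObject and spawns a replacement at MouldLocation, with no change check in this graph.
; SetCurrentMould is an empty stub here.
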(event `self.ReceiveTick`
  (params (DeltaSeconds :type "Float (single-precision)"))
  (bind _currentmould (`self.CurrentMould`))
  (bind _mouldobject (`self.MouldObject`))
  (bind _mouldobject_2 (`self.MouldObject`))
  (bind _mouldobject_3 (`self.MouldObject`))
  (bind (_value _returnvalue) (`BlueprintMapLibrary.Map_Find` (`self.FancyMap`) (`self.CurrentMould`)))
  (`self.UpdateWidget`)
  (`self.CALL_AT_START_OF_TICK`)
  (if _returnvalue
    (if (`KismetStringLibrary.EqualEqual_StrStr` _currentmould "BP_SpearHeadMould_C")
      (if (!= _mouldobject_3 null)
        (`self.K2_DestroyActor` _mouldobject_3))
      (bind _returnvalue_2 (`|SpawnActorFromClass` _value (`KismetMathLibrary.MakeTransform` (`SceneComponent.K2_GetComponentLocation` (`self.MouldLocation`))) "Undefined" "OverrideRootScale" null null))
      (set `self.MouldObject` _returnvalue_2)
      (elif (`KismetStringLibrary.EqualEqual_StrStr` _currentmould "BP_BladeMould_C")
        (if (!= _mouldobject_2 null)
          (`self.K2_DestroyActor` _mouldobject_2))
        (bind _returnvalue_3 (`|SpawnActorFromClass` _value (`KismetMathLibrary.MakeTransform` (`SceneComponent.K2_GetComponentLocation` (`self.MouldLocation`))) "Undefined" "OverrideRootScale" null null))
        (set `self.MouldObject` _returnvalue_3)
        (elif (`KismetStringLibrary.EqualEqual_StrStr` _currentmould "BP_BigBladeMould_C")
          (if (!= _mouldobject null)
            (`self.K2_DestroyActor` _mouldobject))
          (bind _returnvalue_4 (`|SpawnActorFromClass` _value (`KismetMathLibrary.MakeTransform` (`SceneComponent.K2_GetComponentLocation` (`self.MouldLocation`))) "Undefined" "OverrideRootScale" null null))
          (set `self.MouldObject` _returnvalue_4))))))

(fn `SetCurrentMould`)

(fn `UserConstructionScript`
  (`parent.UserConstructionScript`))