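; BP_TableSaw is a converter that shows its processing state through WoodLog and Stick component visibility.
; Each tick it updates its widget and calls CALLATSTARTOFTICK.
; WoodLog hides once Progress reaches 50 and reappears below that while raw input is present, with no explicit hide for empty input.
; Stick and its children show only while processed output is not empty.
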(event `self.ReceiveTick`
  (params (DeltaSeconds :type "Float (single-precision)"))
  (`self.UpdateWidget`)
  (if (>= (`self.Progress`) 50.0)
    (`SceneComponent.SetVisibility` (`self.WoodLog`) false false))
  (`self.CALL_AT_START_OF_TICK`)
  (bind _out (`self.IsProcessedOutputEmpty`))
  (if _out
    (`SceneComponent.SetVisibility` (`self.Stick`) false true)
    (else
      (`SceneComponent.SetVisibility` (`self.Stick`) true true)))
  (bind _out_2 (`self.IsRawInputEmpty`))
  (if _out_2
    _
    (elif (not (>= (`self.Progress`) 50.0))
      (`SceneComponent.SetVisibility` (`self.WoodLog`) true false))))

(fn `UserConstructionScript`)