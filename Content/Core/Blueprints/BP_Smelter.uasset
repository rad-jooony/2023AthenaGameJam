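; BP_Smelter is an automatic smelter building that advances a progress value while it holds raw input.
; Each Tick calls shared start-of-tick logic, then raises Progress by a fixed step until it hits a cap, debug-printing the value.
; A point light shows while progress advances and hides at the cap.
; The molten iron component is visible only while processed output is present.
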(event `self.ReceiveTick`
  (params (DeltaSeconds :type "Float (single-precision)"))
  (if (>= (`self.Progress`) 50.0)
    (`SceneComponent.SetVisibility` (`self.PointLight`) false false))
  (`self.CALL_AT_START_OF_TICK`)
  (bind _out (`self.IsProcessedOutputEmpty`))
  (if _out
    (`SceneComponent.SetVisibility` (`self.MoltenIron`) false false)
    (else
      (`SceneComponent.SetVisibility` (`self.MoltenIron`) true false)))
  (bind _out_2 (`self.IsRawInputEmpty`))
  (if _out_2
    _
    (elif (not (>= (`self.Progress`) 50.0))
      (`self.IncreaseProgress`)
      (`SceneComponent.SetVisibility` (`self.PointLight`) true false))))

(fn `IncreaseProgress`
  (bind _output_get (set `self.Progress` (+ (`self.Progress`) 0.5)))
  (`KismetSystemLibrary.PrintString` (`KismetStringLibrary.Conv_DoubleToString` _output_get) true true (struct :`G` 0.66 :`B` 1.0 :`A` 1.0) 0.0))

(fn `UserConstructionScript`
  (set `self.IsAutomatic` true))