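; BP_HiltMaker is a processing-machine Blueprint, apparently for making hilts, that relies on functions and state defined outside this graph.
; Each Tick it calls CALLATSTARTOFTICK, refreshes its widget, then checks Progress against a threshold, with no action after the check.
; An unconnected branch tests for empty processed output and raw input but never runs.
; BeginPlay and overlap events are disabled, and the construction script only calls the parent.
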(event `self.ReceiveTick`
  (params (DeltaSeconds :type "Float (single-precision)"))
  (`self.CALL_AT_START_OF_TICK`)
  (`self.UpdateWidget`)
  (if (>= (`self.Progress`) 50.0)
    _))

(fn `UserConstructionScript`
  (`parent.UserConstructionScript`))